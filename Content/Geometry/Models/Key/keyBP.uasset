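; Pickup key actor that grants the player's ThirdPersonCharacter HasKey when collected with the Interact input.
; Box overlap by the character shows an interaction prompt, enables input and opens a Gate; leaving reverses all three.
; Interact flashes the prompt's pressed state, then through the Gate sets HasKey, destroys the box and mesh, and briefly shows a "Key picked" message before destroying the actor.
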(event `InputAction|Interact`
  (params (Key :type "Key Structure"))
  (:`Pressed`
    (set `/Game/ThirdPersonBP/Interaction_Widget.is_pressed` true (stale `self.Box.OnComponentBeginOverlap` _returnvalue))
    (`KismetSystemLibrary.Delay` 0.2)
    (set `/Game/ThirdPersonBP/Interaction_Widget.is_pressed` false (stale `self.Box.OnComponentBeginOverlap` _returnvalue))
    (`/Engine/EditorBlueprintResources/StandardMacros.Gate` true :!label _label
      (:`Exit`
        (bind _asthird_person_character (cast `/Game/ThirdPersonBP/Blueprints/ThirdPersonCharacter` (`GameplayStatics.GetPlayerCharacter` 0)))
        (set `/Game/ThirdPersonBP/Blueprints/ThirdPersonCharacter.has_key` true _asthird_person_character)
        (`ActorComponent.K2_DestroyComponent` (`self.Box`))
        (`ActorComponent.K2_DestroyComponent` (`self.StaticMesh`))
        (`KismetSystemLibrary.Delay` 0.2)
        (bind _returnvalue (`|CreateWidget` "/Game/UI/MessageWidget.MessageWidget_C"))
        (set `/Game/UI/MessageWidget.text_interaction` "Key picked" _returnvalue)
        (`UserWidget.AddToViewport` _returnvalue 0)
        (`KismetSystemLibrary.Delay` 0.4)
        (`Widget.RemoveFromParent` _returnvalue)
        (`self.K2_DestroyActor`)))))

(event `self.Box.OnComponentBeginOverlap`
  (params (OverlappedComponent :type "PrimitiveComponent Object Reference") (OtherActor :type "Actor Object Reference") (OtherComp :type "PrimitiveComponent Object Reference") (OtherBodyIndex :type Integer) (bFromSweep :type Boolean) (SweepResult :type "HitResult Structure (by ref)"))
  (cast `/Game/ThirdPersonBP/Blueprints/ThirdPersonCharacter` OtherActor)
  (bind _returnvalue (`|CreateWidget` "/Game/ThirdPersonBP/Interaction_Widget.Interaction_Widget_C"))
  (set `/Game/ThirdPersonBP/Interaction_Widget.interaction_text` "Press 'E' to Pick" _returnvalue)
  (`UserWidget.AddToViewport` _returnvalue 0)
  (`self.EnableInput` (`GameplayStatics.GetPlayerController` 0))
  (goto _label :!via `Open`))

(event `self.Box.OnComponentEndOverlap`
  (params (OverlappedComponent :type "PrimitiveComponent Object Reference") (OtherActor :type "Actor Object Reference") (OtherComp :type "PrimitiveComponent Object Reference") (OtherBodyIndex :type Integer))
  (cast `/Game/ThirdPersonBP/Blueprints/ThirdPersonCharacter` OtherActor)
  (`Widget.RemoveFromParent` (stale `self.Box.OnComponentBeginOverlap` _returnvalue))
  (`self.DisableInput` (`GameplayStatics.GetPlayerController` 0))
  (goto _label :!via `Close`))

(fn `UserConstructionScript`)