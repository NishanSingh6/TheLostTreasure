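; An entrance door Blueprint that stays locked until its OpenDoor event is triggered.
; OpenDoor plays the Final_door timeline, which drives the static mesh's yaw and sets IsActivated.
; While the door is not activated, a ThirdPersonCharacter entering the box trigger gets a "Door Locked" message widget.
; Leaving the box removes that widget, provided the door is still not activated.
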(event `OpenDoor`
  (bind (_direction _newtrack_0) (`Timeline|final_door`)
    (:`Update`
      (`SceneComponent.K2_SetRelativeRotation` (`self.StaticMesh`) (`KismetMathLibrary.MakeRotator` 0.0 0.0 _newtrack_0) false false)
      (set `self.is_activated` true))))

(event `self.Box.OnComponentBeginOverlap`
  (params (OverlappedComponent :type "PrimitiveComponent Object Reference") (OtherActor :type "Actor Object Reference") (OtherComp :type "PrimitiveComponent Object Reference") (OtherBodyIndex :type Integer) (bFromSweep :type Boolean) (SweepResult :type "HitResult Structure (by ref)"))
  (cast `/Game/ThirdPersonBP/Blueprints/ThirdPersonCharacter` OtherActor)
  (if (not (`self.is_activated`))
    (bind _returnvalue (`|CreateWidget` "/Game/UI/MessageWidget.MessageWidget_C"))
    (set `/Game/UI/MessageWidget.text_interaction` "Door Locked" _returnvalue)
    (`UserWidget.AddToViewport` _returnvalue 0)))

(event `self.Box.OnComponentEndOverlap`
  (params (OverlappedComponent :type "PrimitiveComponent Object Reference") (OtherActor :type "Actor Object Reference") (OtherComp :type "PrimitiveComponent Object Reference") (OtherBodyIndex :type Integer))
  (cast `/Game/ThirdPersonBP/Blueprints/ThirdPersonCharacter` OtherActor)
  (if (not (`self.is_activated`))
    (`Widget.RemoveFromParent` (stale `self.Box.OnComponentBeginOverlap` _returnvalue))))

(fn `UserConstructionScript`)