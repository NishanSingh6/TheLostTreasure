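; ChestBP is an interactable chest that the player opens by pressing the Interact input while standing in its trigger box.
; Box overlap by the ThirdPersonCharacter shows an interaction prompt widget, enables input and opens a gate; leaving reverses this.
; Interact flags the widget as pressed, then after a short delay passes the gate to play a timeline rotating the lid pivot, removing the prompt and marking it opened.
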(event `InputAction|Interact`
  (params (Key :type "Key Structure"))
  (:`Pressed`
    (set `/Game/ThirdPersonBP/Interaction_Widget.is_pressed` true (stale `self.Box.OnComponentBeginOverlap` _returnvalue))
    (`KismetSystemLibrary.Delay` 0.2)
    (set `/Game/ThirdPersonBP/Interaction_Widget.is_pressed` true (stale `self.Box.OnComponentBeginOverlap` _returnvalue))
    (`/Engine/EditorBlueprintResources/StandardMacros.Gate` true :!label _label
      (:`Exit`
        (bind (_direction _newtrack_0) (`Timeline|chest_open`)
          (:`Update`
            (`SceneComponent.K2_SetRelativeRotation` (`self.pivot`) (`KismetMathLibrary.MakeRotator` _newtrack_0) false false)
            (`Widget.RemoveFromParent` (stale `self.Box.OnComponentBeginOverlap` _returnvalue))
            (set `self.is_opened` true)))))))

(event `self.Box.OnComponentBeginOverlap`
  (params (OverlappedComponent :type "PrimitiveComponent Object Reference") (OtherActor :type "Actor Object Reference") (OtherComp :type "PrimitiveComponent Object Reference") (OtherBodyIndex :type Integer) (bFromSweep :type Boolean) (SweepResult :type "HitResult Structure (by ref)"))
  (cast `/Game/ThirdPersonBP/Blueprints/ThirdPersonCharacter` OtherActor)
  (if (not (`self.is_opened`))
    (bind _returnvalue (`|CreateWidget` "/Game/ThirdPersonBP/Interaction_Widget.Interaction_Widget_C"))
    (set `/Game/ThirdPersonBP/Interaction_Widget.interaction_text` "Press 'E' To Open" _returnvalue)
    (`UserWidget.AddToViewport` _returnvalue 0)
    (`self.EnableInput` (`GameplayStatics.GetPlayerController` 0))
    (goto _label :!via `Open`)))

(event `self.Box.OnComponentEndOverlap`
  (params (OverlappedComponent :type "PrimitiveComponent Object Reference") (OtherActor :type "Actor Object Reference") (OtherComp :type "PrimitiveComponent Object Reference") (OtherBodyIndex :type Integer))
  (cast `/Game/ThirdPersonBP/Blueprints/ThirdPersonCharacter` OtherActor)
  (if (not (`self.is_opened`))
    (`Widget.RemoveFromParent` (stale `self.Box.OnComponentBeginOverlap` _returnvalue))
    (`self.DisableInput` (`GameplayStatics.GetPlayerController` 0))
    (goto _label :!via `Close`)))

(fn `UserConstructionScript`)