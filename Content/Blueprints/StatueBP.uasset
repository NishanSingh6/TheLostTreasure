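; StatueBP is an interactable statue that rotates on a key press and opens the entrance doors.
; Overlapping its box shows an interaction widget, enables input and opens a gate for the Interact action.
; Each press flashes the widget, then a FlipFlop alternates the timeline forward and backward to yaw the pivot.
; The first timeline update opens the first EnteranceDoorBP and EnteranceDoorBP_2 found, guarded by IsOpened to run once.
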(event `InputAction|Interact`
  (params (Key :type "Key Structure"))
  (:`Pressed`
    (set `/Game/ThirdPersonBP/Interaction_Widget.is_pressed` true (stale `self.Box.OnComponentBeginOverlap` _returnvalue))
    (`KismetSystemLibrary.Delay` 0.2)
    (set `/Game/ThirdPersonBP/Interaction_Widget.is_pressed` false (stale `self.Box.OnComponentBeginOverlap` _returnvalue))
    (`/Engine/EditorBlueprintResources/StandardMacros.Gate` true :!label _label
      (:`Exit`
        (`/Engine/EditorBlueprintResources/StandardMacros.FlipFlop`
          (:`A`
            (bind (_direction _newtrack_0) (`Timeline|rotate_statue` :!via `PlayFromStart` :!label _label_2)
              (:`Update`
                (`SceneComponent.K2_SetRelativeRotation` (`self.pivot`) (`KismetMathLibrary.MakeRotator` 0.0 0.0 _newtrack_0) false false)
                (if (not (`self.is_opened`))
                  (bind _outactors (`GameplayStatics.GetAllActorsOfClass` "/Game/Blueprints/enteranceDoorBP.enteranceDoorBP_C"))
                  (`/Game/Blueprints/enteranceDoorBP.OpenDoor` (`|GetArrayItem` _outactors))
                  (bind _outactors_2 (`GameplayStatics.GetAllActorsOfClass` "/Game/Blueprints/enteranceDoorBP_2.enteranceDoorBP_2_C"))
                  (`/Game/Blueprints/enteranceDoorBP_2.OpenDoor` (`|GetArrayItem` _outactors_2))
                  (set `self.is_opened` true)))))
          (:`B`
            (goto _label_2 :!via `ReverseFromEnd`)))))))

(event `self.Box.OnComponentBeginOverlap`
  (params (OverlappedComponent :type "PrimitiveComponent Object Reference") (OtherActor :type "Actor Object Reference") (OtherComp :type "PrimitiveComponent Object Reference") (OtherBodyIndex :type Integer) (bFromSweep :type Boolean) (SweepResult :type "HitResult Structure (by ref)"))
  (cast `/Game/ThirdPersonBP/Blueprints/ThirdPersonCharacter` OtherActor)
  (bind _returnvalue (`|CreateWidget` "/Game/ThirdPersonBP/Interaction_Widget.Interaction_Widget_C"))
  (`UserWidget.AddToViewport` _returnvalue 0)
  (`self.EnableInput` (`GameplayStatics.GetPlayerController` 0))
  (goto _label :!via `Open`))

(event `self.Box.OnComponentEndOverlap`
  (params (OverlappedComponent :type "PrimitiveComponent Object Reference") (OtherActor :type "Actor Object Reference") (OtherComp :type "PrimitiveComponent Object Reference") (OtherBodyIndex :type Integer))
  (cast `/Game/ThirdPersonBP/Blueprints/ThirdPersonCharacter` OtherActor)
  (`Widget.RemoveFromParent` (stale `self.Box.OnComponentBeginOverlap` _returnvalue))
  (`self.DisableInput` (`GameplayStatics.GetPlayerController` 0))
  (goto _label :!via `Close`))

(fn `UserConstructionScript`)